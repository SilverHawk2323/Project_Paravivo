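; Boss enemy Blueprint that specializes a parent enemy with a smash attack and its own combat ranges.
; Attack runs the parent logic, then calls BossSmashAttack on the BPCAttacks component.
; GetIdealRange returns fixed attack and defend radii, and ReserveAttackToken always returns false.
; The remaining health, damage, team, movement, patrol and attack-state overrides simply forward to the parent.
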(event Custom|ReturnAttackToken_1
  (params (Amount :type Integer)))

(event EventBeginPlay
  (|CallParentFunction) ; This node is disabled and will not be called.\nDrag off pins to build functionality.
)

(event Collision|EventActorBeginOverlap
  (params (OtherActor :type Actor%20Object%20Reference)))

(event EventTick
  (params (DeltaSeconds :type Float%20%28single-precision%29)))

(event EventAttackEnd
  (params (AttackTarget :type Actor%20Object%20Reference))
  (|CallParentFunction AttackTarget))

(event EventStoreAttackTokens
  (params (AttackTarget :type Actor%20Object%20Reference) (Amount :type Integer))
  (|CallParentFunction AttackTarget Amount))

(event EventAttack
  (params (AttackTarget :type Actor%20Object%20Reference))
  (|CallParentFunction AttackTarget)
  (Default|BossSmashAttack (Variables|Default|GetBPC_Attacks) self (Variables|Default|GetAttack%20Info)))

(event EventReturnAttackToken
  (params (Amount :type Integer))
  (|CallParentFunction Amount))

(fn ConstructionScript
  (|CallParentFunction))

(fn GetTeamNumber
  (bind _teamnumber (|CallParentFunction))
  (return _teamnumber))

(fn AttackStart
  (params (AttackTarget :type Actor%20Object%20Reference) (TokensNeeded :type Integer))
  (bind _success (|CallParentFunction AttackTarget TokensNeeded))
  (return _success))

(fn GetIdealRange
  (|CallParentFunction)
  (return 2e+02 4e+02))

(fn ReserveAttackToken
  (params (Amount :type Integer))
  (return false))

(fn IsAttacking
  (bind _attacking (|CallParentFunction))
  (return _attacking))

(fn IsDead
  (bind _dead (|CallParentFunction))
  (return _dead))

(fn Heal
  (params (Amount :type Float%20%28double-precision%29))
  (bind _new_health (|CallParentFunction Amount))
  (return _new_health))

(fn SetMovementSpeed
  (params (Speed :type E_MovementSpeed%20Enum :default "NewEnumerator2"))
  (bind _speedvalue (|CallParentFunction Speed))
  (return _speedvalue))

(fn GetPatrolRoute
  (bind _patrolroute (|CallParentFunction))
  (return _patrolroute))

(fn TakeDamage
  (params (DamageInfo :type S%20Damage%20Info%20Structure) (Damage%20Causer :type Actor%20Object%20Reference))
  (bind _wasdamaged (|CallParentFunction DamageInfo Damage%20Causer))
  (return _wasdamaged))

(fn GetMaxHealth
  (bind _maxhealth (|CallParentFunction))
  (return _maxhealth))

(fn GetCurrentHealth
  (bind _health (|CallParentFunction))
  (return _health))