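; Melee enemy character Blueprint that extends a parent enemy with short and long range attacks and blocking, and is granted GA_Punch on BeginPlay.
; Short attacks run random-length combos via BPCAttacks; long attacks launch it along an arc toward the target and sphere-trace damage.
; Blockable damage skips parent handling and rolls a timed block, with a montage on successful blocks.
; Ending a block returns reserved attack tokens.
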(event OnBlocked(BPC_DamageSystem)
  (params (CanBeParried :type Boolean))
  ;[0.15 0.15 0.15 0.5] Blocking Events
  (Variables|Default|SetBlockingState "NewEnumerator2")
  (Utilities|Time|ClearandInvalidateTimerbyHandle (Variables|Default|GetHoldBlockTimer))
  (Animation|Montage|PlayMontage (Variables|Character|GetMesh) 0
    (:OnCompleted
      _)
    (:OnInterrupted
      _))
  (CallFunction|EndBlock))

(event Custom|LightMeleeAttack
  (params (AttackCount :type Integer))
  ;[0.15 0.15 0.15 0.5] Attack Events
  (if (not (Variables|/Game/Blueprints/ActorComponents/DamageSystem/BPC_DamageSystem.BPC_DamageSystem_C|GetIsDead (Variables|Default|GetBPC_DamageSystem)))
    (Default|LightAttack (Variables|Default|GetBPC_Attacks) AttackCount (Variables|Default|GetDamage%20Info) self)))

(event Custom|StartBlock
  ;[0.15 0.15 0.15 0.5] Blocking Events
  (Utilities|Time|ClearandInvalidateTimerbyHandle (Variables|Default|GetHoldBlockTimer))
  (Components|Movement|StopMovementImmediately (Variables|Character|GetCharacterMovement))
  (Variables|/Game/Blueprints/ActorComponents/DamageSystem/BPC_DamageSystem.BPC_DamageSystem_C|SetIsBlocking (Variables|Default|GetBPC_DamageSystem) true)
  (Variables|Default|SetBlockingState "NewEnumerator1")
  (Components|Movement|StopMovementImmediately (Variables|Character|GetCharacterMovement))
  (bind _returnvalue (Utilities|Time|SetTimerbyEvent (EventDispatchers|CreateEvent :!event Custom|EndBlock) 2.0))
  (Variables|Default|SetHoldBlockTimer _returnvalue))

(event Custom|EndBlock
  ;[0.15 0.15 0.15 0.5] Blocking Events
  (Variables|Default|SetBlockingState "NewEnumerator0")
  (Variables|/Game/Blueprints/ActorComponents/DamageSystem/BPC_DamageSystem.BPC_DamageSystem_C|SetIsBlocking (Variables|Default|GetBPC_DamageSystem) false)
  (bind _keys (Utilities|Map|Keys (Variables|Default|GetReservedAttackTokens)))
  (for _array_element _keys
    (Class|BPIOldDamageable|ReturnAttackToken(Message) _array_element (.Value (Utilities|Map|Find (Variables|Default|GetReservedAttackTokens) _array_element))))
  (Default|CallOnBlockEnded))

(event Custom|ShortRangeAttack
  (params (AttackTarget :type Actor%20Object%20Reference))
  (CallFunction|LightMeleeAttack (Math|Random|RandomIntegerinRange 1 (Variables|Default|GetMax%20Attack%20Count))))

(event Custom|LongRangeAttack
  (params (AttackTarget :type Actor%20Object%20Reference))
  (bind _notifyname (Animation|Montage|PlayMontage (Variables|Character|GetMesh) 0 1.0 0.0 "None" false)
    (:then
      (Variables|/Game/Blueprints/ActorComponents/DamageSystem/BPC_DamageSystem.BPC_DamageSystem_C|SetIsInterruptible (Variables|Default|GetBPC_DamageSystem) true)
      (CallFunction|JumptoAttackTarget AttackTarget)
      (CallFunction|SphereTraceDamage :!label _label))
    (:OnCompleted
      (CallFunction|AttackEnd AttackTarget :!label _label_2)
      (Variables|/Game/Blueprints/ActorComponents/DamageSystem/BPC_DamageSystem.BPC_DamageSystem_C|SetIsInterruptible (Variables|Default|GetBPC_DamageSystem) false))
    (:OnInterrupted
      (goto _label_2))
    (:OnNotifyBegin
      (switch name _notifyname
        (:Slash
          (goto _label))))))

(event Custom|SphereTraceDamage
  (bind _returnvalue (Transformation|GetActorLocation))
  (bind (_outhits _returnvalue_2) (Collision|MultiSphereTraceForObjects _returnvalue (+ _returnvalue (* (Transformation|GetActorForwardVector) 2e+02)) 2e+01 (Utilities|Array|MakeArray "ObjectTypeQuery3") false (Utilities|Array|MakeArray (Components|GetOwner)) "ForDuration"))
  (if _returnvalue_2
    (Default|DamageAllNonTeamMembers (Variables|Default|GetBPC_Attacks) _outhits (Variables|Default|GetDamage%20Info))))

(event Custom|JumpToAttackTarget
  (params (AttackTarget :type Actor%20Object%20Reference))
  (bind _returnvalue (Transformation|GetActorLocation AttackTarget))
  (bind _outlaunchvelocity (Game|SuggestProjectileVelocityCustomArc (Transformation|GetActorLocation) (Math|Vector|MakeVector (.x _returnvalue) (.y _returnvalue) (+ (.z _returnvalue) 2e+02)) 0.0 0.5))
  (Character|LaunchCharacter _outlaunchvelocity false false))

(event EventBeginPlay
  (|CallParentFunction)
  (GameplayAbilities|GiveAbility (Variables|Default|GetAbilitySystem) "/Game/Blueprints/ActorComponents/AttackSystem/GA_Punch.GA_Punch_C" 0 -1))

(event EventAttackEnd
  (params (AttackTarget :type Actor%20Object%20Reference))
  (|CallParentFunction AttackTarget))

(event EventCountered
  (|CallParentFunction))

(event EventApplyDamageEffect
  (params (Damage%20Location :type Vector :default "0, 0, 0") (Damage%20Impulse :type Vector :default "0, 0, 0"))
  (|CallParentFunction Damage%20Location Damage%20Impulse))

(event EventCheckCombo
  (bind _result (Math|Integer|IncrementInt (Variables|Default|GetCurrent%20Combo%20Attack))
    (:%20%20
      (if (< _result (Variables|Default|GetTarget%20Combo%20Count))
        (Ability|Animation|MontageJumptoSection (Components|SkeletalMesh|GetAnimInstance (Variables|Character|GetMesh)) (Utilities|Array|Get(acopy) (Variables|Default|GetCombo%20Section%20Names) (Variables|Default|GetCurrent%20Combo%20Attack)) (Variables|Default|GetCombo%20Attack%20Montage))))))

(event EventAttack
  (params (AttackTarget :type Actor%20Object%20Reference))
  ;[0.15 0.15 0.15 0.5] Attack Events
  (if (not (Variables|Default|GetAttacking))
    (Variables|Default|SetAttacking true)
    (Variables|Default|SetTarget%20Combo%20Count (Math|Random|RandomIntegerinRange 1 (Utilities|Array|Length (Variables|Default|GetCombo%20Section%20Names))))
    (Variables|Default|SetCurrent%20Combo%20Attack 0)
    (Animation|Montage|PlayMontage (Variables|Character|GetMesh) (Utilities|Struct|BreakS_AttackInfo (Variables|Default|GetAttackInfo)) 0.6
      (:OnCompleted
        _)
      (:OnInterrupted
        _))
    (Default|CallOnAttackEnd)
    (Variables|Default|SetAttacking false)))

(event EventCounterWindowOpening
  (|CallParentFunction))

(event EventDoAttackTrace
  (params (Damage%20Source%20Bone :type Name :default "None"))
  (|CallParentFunction Damage%20Source%20Bone))

(event EventEnableActor
  (|CallParentFunction))

(event EventDeathEvent
  (|CallParentFunction))

(event EventCounterWindowClosed
  (|CallParentFunction))

(fn ConstructionScript
  (|CallParentFunction))

(fn TrytoBlock
  (if (<= (Math|Random|RandomFloat) (Variables|Default|GetBlockChance))
    (CallFunction|StartBlock)))

(fn GetIdealRange
  (return 1e+02 4e+02))

(fn TakeDamage
  (params (DamageInfo :type S%20Damage%20Info%20Structure) (Damage%20Causer :type Actor%20Object%20Reference))
  (if (Utilities|Struct|BreakS_DamageInfo DamageInfo)
    (CallFunction|TrytoBlock)
    (return false)
    (else
      (bind _wasdamaged (|CallParentFunction DamageInfo Damage%20Causer))
      (return _wasdamaged))))