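; Mage enemy AI character that attacks with dark magic, teleports and supplies its own ideal attack and defend ranges.
; Attack plays a montage whose Fire notify triggers the dark magic through BPCAttacks; the lightning strike event exists but Attack does not call it.
; Teleport is a fast, invisible flying AI move with particle effects and pawn collision ignored, restoring walking, visibility and collision on success or failure.
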(event Custom|MageAttack
  (params (AttackTarget :type Actor%20Object%20Reference))
  (Default|LightingStrike (Variables|Default|GetBPC_Attacks) 0.2 AttackTarget (.amount (Variables|Default|GetLighting%20Attack%20Info)))
  (Utilities|FlowControl|Delay 0.2)
  (CallFunction|AttackEnd AttackTarget))

(event Custom|Teleport
  (params (Location :type Vector))
  (bind _charactermovement (Variables|Character|GetCharacterMovement))
  (bind _mesh (Variables|Character|GetMesh))
  (if (not (Variables|Default|GetIsTeleporting))
    (Variables|Default|SetIsTeleporting true)
    (Pawn|Components|CharacterMovement|SetMovementMode _charactermovement "MOVE_Flying" 0)
    (Variables|/Script/Engine.CharacterMovementComponent|SetMaxFlySpeed _charactermovement 2e+03)
    (Variables|/Script/Engine.CharacterMovementComponent|SetMaxAcceleration _charactermovement 999999.0)
    (Rendering|SetVisibility (Variables|Character|GetMesh) false true)
    (Collision|SetCollisionResponsetoChannel (Variables|Default|GetCapsuleComponent) "ECC_Pawn" "ECR_Ignore")
    (bind _returnvalue (Effects|SpawnEmitterAttached 0 _mesh "pelvis"))
    (Variables|Default|SetTeleportBodyEffect _returnvalue)
    (bind _returnvalue_2 (Effects|SpawnEmitterAttached 0 _mesh "pelvis"))
    (Variables|Default|SetTeleportTrailEffect _returnvalue_2)
    (Animation|StopAnimMontage 0)
    (AI|AIMoveTo self Location 0 15.0 false
      (:OnSuccess
        _)
      (:OnFail
        _))
    (CallFunction|TeleportEnd)
    (else
      (Utilities|FlowControl|DelayUntilNextTick)
      (Default|CallOnTeleportEnd))))

(event Custom|TeleportEnd
  (bind _charactermovement (Variables|Character|GetCharacterMovement))
  (Components|Movement|StopMovementImmediately _charactermovement)
  (Pawn|Components|CharacterMovement|SetMovementMode _charactermovement "MOVE_Walking" 0)
  (Variables|/Script/Engine.CharacterMovementComponent|SetMaxAcceleration _charactermovement 1.5e+03)
  (Rendering|SetVisibility (Variables|Character|GetMesh) true true)
  (Collision|SetCollisionResponsetoChannel (Variables|Default|GetCapsuleComponent) "ECC_Pawn" "ECR_Block")
  (Default|CallOnTeleportEnd)
  (Utilities|FlowControl|Delay 0.5)
  (Variables|Default|SetIsTeleporting false)
  (Utilities|FlowControl|Sequence
    (:then_0
      (bind _teleportbodyeffect (Variables|Default|GetTeleportBodyEffect)
        (:then
          (Components|DestroyComponent _teleportbodyeffect))
        (:else)))
    (:then_1
      (bind _teleporttraileffect (Variables|Default|GetTeleportTrailEffect)
        (:then
          (Components|DestroyComponent _teleporttraileffect))
        (:else)))))

(event Custom|DarkMagicAttack
  (params (AttackTarget :type Actor%20Object%20Reference))
  (bind _notifyname (Animation|Montage|PlayMontage (Variables|Character|GetMesh) 0)
    (:OnCompleted
      (CallFunction|AttackEnd AttackTarget :!label _label))
    (:OnInterrupted
      (goto _label))
    (:OnNotifyBegin
      (switch name _notifyname
        (:Fire
          (Default|DarkMagicAttack (Variables|Default|GetBPC_Attacks) (Math|Transform|MakeTransform (+ (Transformation|GetActorLocation) (* (Transformation|GetActorForwardVector) 1.2e+02)) (Transformation|GetActorRotation)) AttackTarget (Variables|Default|GetAttack%20Info)))))))

(event EventBeginPlay
  (|CallParentFunction) ; This node is disabled and will not be called.\nDrag off pins to build functionality.
)

(event Collision|EventActorBeginOverlap
  (params (OtherActor :type Actor%20Object%20Reference)))

(event EventTick
  (params (DeltaSeconds :type Float%20%28single-precision%29)))

(event EventAttack
  (params (AttackTarget :type Actor%20Object%20Reference))
  (|CallParentFunction AttackTarget)
  (CallFunction|DarkMagicAttack AttackTarget))

(event EventDeath)

(fn ConstructionScript
  (|CallParentFunction))

(fn GetIdealRange
  (return 4e+02 6e+02))