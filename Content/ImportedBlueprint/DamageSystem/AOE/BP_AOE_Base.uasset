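; BP_AOE_Base is a base area-of-effect actor for the damage system that finds pawns within a radius of its location.
; Trigger runs on demand, or after a short delay from BeginPlay when TriggerOnBeginPlay is set.
; It performs a sphere overlap with optional instigator exclusion and debug drawing, then passes the results to OnAOEOverlapActor.
; It applies no damage itself; a leftover debug print reads from a disconnected loop.
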(event Custom|SpawnAOESphere
  (if (not (Variables|Default|GetDrawDebug))
    _
    (else
      (Rendering|Debug|DrawDebugSphere (Transformation|GetActorLocation) (Variables|Default|GetRadius) 12 "(R=1.000000,G=0.000000,B=0.884676,A=1.000000)" 2.0 1.0)))
  (bind _outactors (Collision|SphereOverlapActors (Transformation|GetActorLocation) (Variables|Default|GetRadius) (Utilities|Array|MakeArray "ObjectTypeQuery3") 0 (select (Variables|Default|GetIgnoreInstigator) (Utilities|Array|MakeArray (Game|GetInstigator)) 0)))
  (Default|CallOnAOEOverlapActor _outactors)
  (Development|PrintString (Utilities|GetDisplayName (stale _array_element))))

(event Custom|Trigger
  (CallFunction|SpawnAOESphere))

(event EventBeginPlay
  (if (Variables|Default|GetTriggerOnBeginPlay)
    (Utilities|FlowControl|Delay 0.5)
    (CallFunction|Trigger)))

(fn ConstructionScript)