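; Base Blueprint for an area-of-effect blast actor that adds visual and audio feedback to the parent's Trigger.
; Trigger calls the parent, attaches the emitter effect to the root and plays the blast sound at the actor's location.
; The actor destroys itself when the emitter finishes, or after a short delay if no emitter is set.
; An alternate BlastEffect system spawn is left disconnected and never runs.
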(event Custom|SpawnBlastEffect
  (bind _emitterblasteffect (Variables|Default|GetEmitterBlastEffect)
    (:then
      (bind _returnvalue (Effects|SpawnEmitterAttached _emitterblasteffect (Variables|Default|GetDefaultSceneRoot) "None"))
      (EventDispatchers|BindEventtoOnSystemFinished _returnvalue (delegate Custom|SystemFinished)))
    (:else
      (Utilities|FlowControl|Delay 1.0)
      (Actor|DestroyActor))))

(event Custom|SpawnBlastSound
  (bind _blast_sound (Variables|Default|GetBlast%20Sound)
    (:then
      (Audio|PlaySoundatLocation _blast_sound (Transformation|GetActorLocation) "0, 0, 0" 1.0 1.0 0.0 0 0 0 0))
    (:else)))

(event Custom|SystemFinished
  (params (PSystem :type Particle%20System%20Component%20Object%20Reference))
  (Actor|DestroyActor))

(event EventBeginPlay
  (|CallParentFunction) ; This node is disabled and will not be called.\nDrag off pins to build functionality.
)

(event EventTrigger
  (|CallParentFunction)
  (CallFunction|SpawnBlastEffect)
  (CallFunction|SpawnBlastSound))

(fn ConstructionScript
  (|CallParentFunction))