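; Attack component that runs boss, minion, light combo, lightning, dark magic and heal actions for combat characters.
; Melee attacks use forward sphere traces, mostly on montage notifies, while light attacks cycle a saveable four-step combo and repeat for non-player owners.
; Spells spawn AOE or projectile actors and bind their overlap or impact events.
; Damage is filtered by team, sent through interface messages, and reported as AI damage events.
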(event Custom|LightingStrike
  (params (DelayBeforeStrike :type Float%20%28single-precision%29) (AttackTarget :type Actor%20Object%20Reference) (DamageAmount :type Float%20%28double-precision%29))
  (bind _returnvalue (Components|GetOwner))
  (bind (_aspawn _bsuccess) (Utilities|Casting|CastToPawn _returnvalue))
  (bind _returnvalue_2 (Game|SpawnActorfromClass "/Game/ImportedBlueprint/DamageSystem/AOE/BP_AOE_LightingStrike.BP_AOE_LightingStrike_C" (Math|Transform|MakeTransform (|IsAttackTargetValid _aspawn AttackTarget) "0, 0, 0" "1.000000,1.000000,1.000000") "Undefined" "MultiplyWithRoot" 0 DelayBeforeStrike AttackTarget 0 2e+02 true false false (select _bsuccess _aspawn 0)))
  (EventDispatchers|BindEventtoOnAOEOverlapActor _returnvalue_2 (delegate Custom|DamageEnemyAOE)))

(event Custom|DamageEnemyAOE
  (params (Actor :type Array%20of%20Actor%20Object%20References))
  (bind _returnvalue (Components|GetOwner))
  (bind _returnvalue_2 (Components|GetOwner))
  (bind (_aspawn _bsuccess) (Utilities|Casting|CastToPawn _returnvalue_2))
  (for _array_element Actor
    (EventDispatchers|UnbindEventfromOnAOEOverlapActor (stale Custom|LightingStrike _returnvalue_2) (delegate Custom|DamageEnemyAOE))
    (bind _teamnumber (Class|BPIOldDamageable|GetTeamNumber(Message) _array_element))
    (bind _teamnumber_2 (Class|BPIOldDamageable|GetTeamNumber(Message) (Components|GetOwner)))
    (if (!= _teamnumber_2 _teamnumber)
      (Class|BPIOldDamageable|TakeDamage(Message) _array_element (Utilities|Struct|MakeS_OldDamageInfo (stale Custom|LightingStrike DamageAmount) "NewEnumerator3" "NewEnumerator1" false false false true) _returnvalue)
      (Class|AISenseDamage|ReportDamageEvent _array_element _returnvalue (stale Custom|LightingStrike DamageAmount) (Transformation|GetActorLocation (select _bsuccess _aspawn 0)) "0, 0, 0" "None"))))

(event Custom|HealTarget
  (params (HealTarget :type Actor%20Object%20Reference))
  (bind _returnvalue (Transformation|GetActorLocation HealTarget))
  (Utilities|IsValid HealTarget
    (:Is%20Valid
      (bind (_outhit _returnvalue_2) (Collision|LineTraceByChannel _returnvalue (* _returnvalue "10.000000,1.000000,-1000.000000") "TraceTypeQuery1" false (Utilities|Array|MakeArray HealTarget) "None"))
      (if _returnvalue_2
        (bind _returnvalue_3 (Game|SpawnActorfromClass "/Game/ImportedBlueprint/DamageSystem/AOE/BP_AOE_Heal.BP_AOE_Heal_C" (Math|Transform|MakeTransform (.Location (Collision|BreakHitResult _outhit)) "0, 0, 0" "1.000000,1.000000,1.000000") "Undefined" "MultiplyWithRoot" 0 1.0 4.0 1.2e+02 false false true 0))
        (EventDispatchers|BindEventtoOnAOEOverlapActor _returnvalue_3 (delegate Custom|OnHealTarget))))))

(event Custom|OnHealTarget
  (params (Actor :type Array%20of%20Actor%20Object%20References))
  (for _array_element Actor
    (if (== _array_element (stale Custom|HealTarget HealTarget))
      (Class|BPIOldDamageable|Heal(Message) _array_element 1e+01))))

(event Custom|LightAttack
  (params (MaxAttacks :type Integer) (LightAttackInfo :type S%20Damage%20Info%20Structure) (Character :type Character%20Object%20Reference))
  (bind _returnvalue (Components|GetOwner))
  (bind (_aspawn _bsuccess) (Utilities|Casting|CastToPawn _returnvalue))
  (Class|AISenseHearing|ReportNoiseEvent (Transformation|GetActorLocation (Components|GetOwner)) 1.0 Character 1e+03 "None")
  (Variables|Default|SetMaxAttacks MaxAttacks)
  (bind _output_get (Variables|Default|SetDamage%20Info LightAttackInfo))
  (bind _hitactor (|AttackAnimation Character)
    (:execute
      (bind _output_get_2 (Variables|Default|SetAttackTarget _hitactor))
      (bind _owner (Variables|Default|GetOwner)
        (:then
          (Class|AISenseDamage|ReportDamageEvent _output_get_2 _owner (.Amount (Utilities|Struct|BreakS_DamageInfo _output_get)) (Transformation|GetActorLocation (select _bsuccess _aspawn 0)) "0, 0, 0" "None")
          (|RepeatLightAttack))
        (:else)))))

(event Custom|DarkMagicAttack
  (params (SpawnTransform :type Transform) (Target :type Actor%20Object%20Reference) (DamageInfo :type S%20Damage%20Info%20Structure))
  (bind _returnvalue (Components|GetOwner))
  (bind _returnvalue_2 (Transformation|GetActorLocation _returnvalue))
  (bind (_outhits _returnvalue_3) (Collision|MultiSphereTraceForObjects _returnvalue_2 (+ _returnvalue_2 (* (Transformation|GetActorForwardVector _returnvalue) 6e+02)) 2e+01 (Utilities|Array|MakeArray "ObjectTypeQuery3") false (Utilities|Array|MakeArray _returnvalue) "ForDuration"))
  (if _returnvalue_3
    (bind _returnvalue_4 (Game|SpawnActorfromClass "/Game/ImportedBlueprint/DamageSystem/Projectiles/BP_Projectile_DarkEnergy.BP_Projectile_DarkEnergy_C" SpawnTransform "Undefined" "MultiplyWithRoot" (Components|GetOwner) 5e+02 0.0 Target (select _returnvalue_3 true false) 0))
    (EventDispatchers|BindEventtoOnProjectileImpact _returnvalue_4 (delegate Custom|DamageEnemy))))

(event Custom|DamageEnemy
  (params (Other%20Actor :type Actor%20Object%20Reference) (Hit :type Hit%20Result%20Structure) (DamageInfo :type S%20Damage%20Info%20Structure))
  (EventDispatchers|UnbindEventfromOnProjectileImpact (stale Custom|DarkMagicAttack _returnvalue_4) (delegate Custom|DamageEnemy))
  (bind _teamnumber (Class|BPIOldDamageable|GetTeamNumber(Message) Other%20Actor))
  (bind _teamnumber_2 (Class|BPIOldDamageable|GetTeamNumber(Message) (Components|GetOwner)))
  (if (!= _teamnumber_2 _teamnumber)
    (bind _damagedactor (CallFunction|DamageFirstNonTeamMember (stale Custom|DarkMagicAttack _outhits) (stale Custom|DarkMagicAttack DamageInfo)))
    (Class|AISenseDamage|ReportDamageEvent _damagedactor (Components|GetOwner) (.Amount (Utilities|Struct|BreakS_DamageInfo (stale Custom|DarkMagicAttack DamageInfo))) (Transformation|GetActorLocation (Components|GetOwner)) "0, 0, 0" "None")
    (Default|CallOnAttackEnded)))

(event Custom|MinionAttack
  (params (AttackInfo :type S%20Damage%20Info%20Structure) (Instigator :type Character%20Object%20Reference))
  (bind _returnvalue (Components|GetOwner))
  (bind (_aspawn _bsuccess) (Utilities|Casting|CastToPawn _returnvalue))
  (bind _output_get (Variables|Default|SetOwner Instigator))
  (Variables|Default|SetDamage%20Info AttackInfo)
  (bind _notifyname (Animation|Montage|PlayMontage (Variables|/Script/Engine.Character|GetMesh _output_get) 0)
    (:OnNotifyBegin
      (switch name _notifyname
        (:Slash
          (bind (_outhit _returnvalue_2) (Collision|SphereTraceForObjects (Transformation|GetActorLocation (Variables|Default|GetOwner)) (+ (Transformation|GetActorLocation (Variables|Default|GetOwner)) (* (Transformation|GetActorForwardVector (Variables|Default|GetOwner)) 2e+02)) 1.5e+02 (Utilities|Array|MakeArray "ObjectTypeQuery3") false (Utilities|Array|MakeArray (Components|GetOwner) (Variables|Default|GetOwner)) "None"))
          (if _returnvalue_2
            (bind _damagedactor (CallFunction|DamageFirstNonTeamMember (Utilities|Array|MakeArray _outhit) (Variables|Default|GetDamage%20Info)))
            (bind _output_get_2 (Variables|Default|SetAttackTarget _damagedactor))
            (Class|AISenseDamage|ReportDamageEvent _output_get_2 (Variables|Default|GetOwner) (.amount (Variables|Default|GetDamage%20Info)) (Transformation|GetActorLocation (select _bsuccess _aspawn 0)) "0, 0, 0" "None")))
        (:AttackEnd
          (Class|BPIEnemyAI|AttackEnd(Message) (Variables|Default|GetOwner) (Variables|Default|GetAttackTarget)))))))

(event Custom|BossSmashAttack
  (params (Character :type Character%20Object%20Reference) (Attack%20info :type S%20Damage%20Info%20Structure))
  (bind _returnvalue (Components|GetOwner))
  (bind (_aspawn _bsuccess) (Utilities|Casting|CastToPawn _returnvalue))
  (bind _output_get (Variables|Default|SetOwner Character))
  (Variables|Default|SetDamage%20Info Attack%20info)
  (bind _notifyname (Animation|Montage|PlayMontage (Variables|/Script/Engine.Character|GetMesh _output_get) 0)
    (:OnNotifyBegin
      (switch name _notifyname
        (:Smash
          (bind (_outhits _returnvalue_2) (Collision|MultiSphereTraceForObjects (Transformation|GetActorLocation (Variables|Default|GetOwner)) (+ (Transformation|GetActorLocation (Variables|Default|GetOwner)) (* (Transformation|GetActorForwardVector (Variables|Default|GetOwner)) 2e+02)) 1.5e+02 (Utilities|Array|MakeArray "ObjectTypeQuery3") false (Utilities|Array|MakeArray (Components|GetOwner) (Variables|Default|GetOwner)) "ForDuration"))
          (if _returnvalue_2
            (bind _actorsdamaged (CallFunction|DamageAllNonTeamMembers _outhits (Variables|Default|GetDamage%20Info)))
            (for _array_element _actorsdamaged
              (bind _output_get_2 (Variables|Default|SetAttackTarget _array_element))
              (bind _owner (Variables|Default|GetOwner)
                (:then
                  (Class|AISenseDamage|ReportDamageEvent _output_get_2 _owner (.Amount (Utilities|Struct|BreakS_DamageInfo (Variables|Default|GetDamage%20Info))) (Transformation|GetActorLocation (select _bsuccess _aspawn 0)) "0, 0, 0" "None"))
                (:else)))))
        (:AttackEnd
          (bind _attacktarget (Variables|Default|GetAttackTarget)
            (:then
              (Class|BPIEnemyAI|AttackEnd(Message) (Variables|Default|GetOwner) _attacktarget))
            (:else)))))))

(fn DamageAllNonTeamMembers
  (params (Hits :type Array%20of%20Hit%20Result%20Structures) (DamageInfo :type S%20Damage%20Info%20Structure))
  (for _array_element Hits
    (bind _teamnumber (Class|BPIOldDamageable|GetTeamNumber(Message) (.HitActor (Collision|BreakHitResult _array_element))))
    (bind _teamnumber_2 (Class|BPIOldDamageable|GetTeamNumber(Message) (Components|GetOwner)))
    (if (and (!= _teamnumber_2 _teamnumber) (not (Utilities|Array|ContainsItem (LocalVariables|GetActorsDamagedSoFar) (.HitActor (Collision|BreakHitResult _array_element)))))
      (Class|BPIDamageable|TakeDamage(Message) (.HitActor (Collision|BreakHitResult _array_element)) DamageInfo (Components|GetOwner))
      (Utilities|Array|AddUnique (LocalVariables|GetActorsDamagedSoFar) (.HitActor (Collision|BreakHitResult _array_element)))))
  (return (LocalVariables|GetActorsDamagedSoFar)))

(fn DamageFirstNonTeamMember
  (params (Hits :type Array%20of%20Hit%20Result%20Structures) (DamageInfo :type S%20Damage%20Info%20Structure))
  (bind _array_element (Utilities|Array|ForEachLoopwithBreak Hits :!label _label)
    (:LoopBody
      (bind _teamnumber (Class|BPIOldDamageable|GetTeamNumber(Message) (.HitActor (Collision|BreakHitResult _array_element))))
      (bind _teamnumber_2 (Class|BPIOldDamageable|GetTeamNumber(Message) (Components|GetOwner)))
      (if (!= _teamnumber_2 _teamnumber)
        (Class|BPIDamageable|TakeDamage(Message) (.HitActor (Collision|BreakHitResult _array_element)) DamageInfo (Components|GetOwner))
        (Utilities|FlowControl|Sequence
          (:then_0
            (goto _label Break))
          (:then_1
            (return (.HitActor (Collision|BreakHitResult _array_element)))))))))

(event Custom|ResetCombo
  (bind _asbp_enemy_base (Utilities|Casting|CastToBP_EnemyBase (Components|GetOwner))
    (:then
      (Default|AttackEnd _asbp_enemy_base (Variables|Default|GetAttackTarget)))
    (:CastFailed
      _))
  (Variables|Default|SetAttackCount 0)
  (Variables|Default|SetSaveAttack false)
  (Variables|Default|SetIsAttacking false))

(event Custom|ComboAttackSave
  (bind _owner (Variables|Default|GetOwner))
  (bind _owner_2 (Variables|Default|GetOwner))
  (bind _returnvalue (Transformation|GetActorLocation _owner_2))
  (if (Variables|Default|GetSaveAttack)
    (Variables|Default|SetSaveAttack false)
    (switch int (Variables|Default|GetAttackCount)
      (:0
        (Variables|Default|SetAttackCount 1)
        (bind _returnvalue_2 (Animation|PlayAnimMontage _owner 0 1.0 "None"))
        (Variables|Default|SetAttackLength _returnvalue_2))
      (:1
        (Variables|Default|SetAttackCount 2)
        (bind _returnvalue_3 (Animation|PlayAnimMontage _owner 0 1.0 "None"))
        (Variables|Default|SetAttackLength _returnvalue_3))
      (:2
        (Variables|Default|SetAttackCount 3)
        (bind _returnvalue_4 (Animation|PlayAnimMontage _owner 0 1.0 "None"))
        (Variables|Default|SetAttackLength _returnvalue_4))
      (:3
        (Variables|Default|SetAttackCount 0)
        (bind _returnvalue_5 (Animation|PlayAnimMontage _owner 0 1.0 "None"))
        (Variables|Default|SetAttackLength _returnvalue_5)))
    (Math|Integer|IncrementInt (Variables|Default|GetTotalAttacksDone)
      (:%20%20
        (bind (_outhits _returnvalue_6) (Collision|MultiSphereTraceForObjects _returnvalue (+ _returnvalue (* (Transformation|GetActorForwardVector _owner_2) 2e+02)) 1.5e+02 (Utilities|Array|MakeArray "ObjectTypeQuery3") false (Utilities|Array|MakeArray (Components|GetOwner) (Variables|Default|GetOwner)) "ForDuration"))
        (if _returnvalue_6
          (bind _actorsdamaged (CallFunction|DamageAllNonTeamMembers _outhits (Variables|Default|GetDamage%20Info)))
          (for _array_element _actorsdamaged
            (return _array_element "")))))))