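; Actor component for the damage system that tracks health, damage, healing and death, plus a pool of attack tokens to reserve and return.
; TakeDamage uses the CanBeDamaged macro to block, apply or ignore hits based on death, invincibility and blocking, then calls blocked, death or interruptible damage-response dispatchers.
; ResetHP and GetHealth read a Gameplay Ability System attribute from the owner, while UpdateHealthBar queries owner messages to set widget percentage.
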(event EventBeginPlay)

(event EventTick
  (params (DeltaSeconds :type Float%20%28single-precision%29)))

(fn Heal
  (params (Amount :type Float%20%28double-precision%29))
  (if (not (Variables|DamageSystem|GetIsDead))
    (bind _output_get (Variables|DamageSystem|SetHealth (Math|Float|Clamp(Float) (+ Amount (Variables|DamageSystem|GetHealth)) 0.0 (Variables|DamageSystem|GetMaxHealth))))
    (return _output_get)))

(fn TakeDamage
  (params (DamageInfo :type S%20Damage%20Info%20Structure) (DamageCauser :type Actor%20Object%20Reference))
  (bind (_amount _damagetype _damageresponse _shoulddamageinvincible _canbeblocked _canbeparried _shouldforceinterrupt) (Utilities|Struct|BreakS_DamageInfo DamageInfo))
  ;[1 1 1] Once an actor takes damage check whether to block, do, or take no damage
  (Utilities|CanbeDamaged _shoulddamageinvincible _canbeblocked
    (:BlockDamage
      (Default|CallOnBlocked _canbeparried)
      (return false))
    (:DoDamage
      (bind _output_get (Variables|DamageSystem|SetHealth (- (Variables|DamageSystem|GetHealth) _amount)))
      (if (<= _output_get 0.0)
        (Variables|DamageSystem|SetIsDead true)
        (Default|CallOnDeath) ; When Called the Actor's Death event triggers
        (return true)
        (elif (or (Variables|DamageSystem|GetIsInterruptible) _shouldforceinterrupt)
          (Default|CallOnDamageResponse _damageresponse DamageCauser)
          (return true))))
    (:NoDamage
      (return false))))

(fn ReserveAttackToken
  (params (Amount :type Integer))
  (if (>= (Variables|DamageSystem|GetAttackTokensCount) Amount)
    (Variables|DamageSystem|SetAttackTokensCount (- (Variables|DamageSystem|GetAttackTokensCount) Amount))
    (return true)
    (else
      (return false))))

(fn ReturnAttackToken
  (params (Amount :type Integer))
  (Variables|DamageSystem|SetAttackTokensCount (+ (Variables|DamageSystem|GetAttackTokensCount) Amount))
  (return))

(fn ResetHP
  (bind _returnvalue (Components|GetOwner))
  (bind _returnvalue_2 (Ability|GetAbilitySystemComponent _returnvalue))
  (bind (_bfound _returnvalue_3) (Class|AbilitySystemComponent|GetGameplayAttributeValue _returnvalue_2 "(AttributeName=\"MaxHealth\",Attribute=/Script/Paravivo.DamageableAttributeSet:MaxHealth,AttributeOwner=\"/Script/CoreUObject.Class'/Script/Paravivo.DamageableAttributeSet'\")"))
  (if _bfound
    (Variables|DamageSystem|SetHealth _returnvalue_3)))

(fn UpdateHealthBar
  (params (Widget :type UI%20Life%20Bar%20Object%20Reference))
  (bind _returnvalue (Components|GetOwner))
  (bind _health (Class|BPIDamageable|GetCurrentHealth(Message) _returnvalue))
  (bind _maxhealth (Class|BPIDamageable|GetMaxHealth(Message) _returnvalue))
  (Default|SetLifePercentage Widget (/ _health _maxhealth)))

(fn GetHealth
  (bind _returnvalue (Components|GetOwner))
  (bind _returnvalue_2 (Ability|GetAbilitySystemComponent _returnvalue))
  (bind (_bfound _returnvalue_3) (Class|AbilitySystemComponent|GetGameplayAttributeValue _returnvalue_2 "(AttributeName=\"Health\",Attribute=/Script/Paravivo.DamageableAttributeSet:Health,AttributeOwner=\"/Script/CoreUObject.Class'/Script/Paravivo.DamageableAttributeSet'\")"))
  (if _bfound
    (return _returnvalue_3)))

(fn SetHealth
  (params (NewHealth :type Float%20%28double-precision%29))
  (Variables|DamageSystem|SetHealth NewHealth))