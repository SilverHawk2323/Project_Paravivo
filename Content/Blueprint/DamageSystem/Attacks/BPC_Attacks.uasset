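; Attack component that detects melee hits from its owning character and delivers damage to the actors hit.
; HitScanStart stores damage info and an effect spec, clears the hit list and starts a looping timer that HitScanEnd clears.
; Punch sphere-traces pawns forward from the damage bone, damaging each target with an Ability System Component and BPI_Damageable once per scan.
; Each hit also reports a damage event for AI perception.
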(fn HitScanStart
  (params (Incoming%20Damage%20Info :type S%20Damage%20Info%20Structure) (EffectSpecHandle :type Gameplay%20Effect%20Spec%20Handle%20Structure))
  (Variables|Default|SetIncoming%20Damage%20Info Incoming%20Damage%20Info)
  (Utilities|Array|Clear (Variables|Default|GetHitActors))
  (Variables|Default|SetEffect%20Spec%20Handle EffectSpecHandle)
  (bind _returnvalue (Utilities|Time|SetTimerbyEvent (EventDispatchers|CreateEvent :!event Punch) 0.033333 true))
  (Variables|Default|SetHitScanTimer _returnvalue))

(fn HitScanEnd
  (Utilities|Time|ClearandInvalidateTimerbyHandle (Variables|Default|GetHitScanTimer)))

(fn Punch
  (bind _returnvalue (Components|GetOwner))
  (bind _ascharacter (Utilities|Casting|CastToCharacter _returnvalue))
  (bind _outhits (Collision|MultiSphereTraceForObjects (Transformation|GetSocketLocation (Variables|/Script/Engine.Character|GetMesh _ascharacter) (Variables|Default|GetDamageBone)) (+ (Transformation|GetSocketLocation (Variables|/Script/Engine.Character|GetMesh _ascharacter) (Variables|Default|GetDamageBone)) (* (Transformation|GetActorForwardVector _ascharacter) (LocalVariables|GetTraceDistance))) 2e+01 (Utilities|Array|MakeArray "ObjectTypeQuery3") false (Utilities|Array|MakeArray _returnvalue) "None" true "(R=1.000000,G=0.000000,B=0.000000,A=1.000000)" "(R=0.000000,G=1.000000,B=0.000000,A=1.000000)" 1.0))
  (for _array_element _outhits
    (Utilities|IsValid (Ability|GetAbilitySystemComponent (.HitActor (Collision|BreakHitResult _array_element)))
      (:Is%20Valid
        (if (Utilities|DoesObjectImplementInterface (.HitActor (Collision|BreakHitResult _array_element)) "/Game/Blueprint/DamageSystem/BPI_Damageable.BPI_Damageable_C")
          (if (not (Utilities|Array|ContainsItem (Variables|Default|GetHitActors) (.HitActor (Collision|BreakHitResult _array_element))))
            (Utilities|Array|AddUnique (Variables|Default|GetHitActors) (.HitActor (Collision|BreakHitResult _array_element)))
            (Class|BPIDamageable|TakeDamage(Message) (.HitActor (Collision|BreakHitResult _array_element)) (Variables|Default|GetIncoming%20Damage%20Info) (Components|GetOwner) (Variables|Default|GetEffect%20Spec%20Handle))
            (Class|AISenseDamage|ReportDamageEvent (.HitActor (Collision|BreakHitResult _array_element)) (Components|GetOwner) 1.0 (Transformation|GetActorLocation (.HitActor (Collision|BreakHitResult _array_element))) "0, 0, 0" "None"))
          (else
            (Development|PrintString "No damageable interface")))))))