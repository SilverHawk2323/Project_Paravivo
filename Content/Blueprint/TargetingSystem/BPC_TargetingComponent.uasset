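; Targeting component for a Character that picks an actor to lock on to and stores it as LockedOnActor.
; A sphere trace around the owner adds pawns tagged Data.Targetable to a candidate list that is never cleared.
; Candidates that pass a pawn-only camera line trace go to selection by a weighted facing and squared-distance score.
; CompareTarget is only assigned to itself, so the best score is never recorded.
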(event Custom|Lock%20On%20To%20Target
  (bind _targetingactors (CallFunction|FindActorstoLockonto))
  (bind _closesttarget (CallFunction|FindClosetTarget _targetingactors))
  (Utilities|IsValid _closesttarget
    (:Is%20Valid
      (Variables|Default|SetLockedOnActor _closesttarget))))

(event EventBeginPlay
  (bind _ascharacter (Utilities|Casting|CastToCharacter (Components|GetOwner)))
  (Variables|Default|SetCharacterRef _ascharacter)
  (Variables|Default|SetCameraRef (Actor|GetComponentbyClass (Variables|Default|GetCharacterRef) "/Script/Engine.CameraComponent")))

(fn FindActorstoLockonto
  (bind _characterref (Variables|Default|GetCharacterRef))
  (bind _potentialtargetingactors (LocalVariables|GetPotentialTargetingActors))
  (bind _returnvalue (Transformation|GetActorLocation _characterref))
  (bind (_outhits _returnvalue_2) (Collision|MultiSphereTraceForObjects _returnvalue _returnvalue (Variables|Default|GetRadius) (Utilities|Array|MakeArray "ObjectTypeQuery3") false (Utilities|Array|MakeArray (Components|GetOwner)) "None"))
  (for _array_element _outhits
    (if (and _returnvalue_2 (GameplayTags|HasMatchingGameplayTag (Ability|GetAbilitySystemComponent (.HitActor (Collision|BreakHitResult _array_element))) "(TagName=\"Data.Targetable\")"))
      (if (not (Utilities|Array|ContainsItem _potentialtargetingactors (.HitActor (Collision|BreakHitResult _array_element))))
        (Utilities|Array|AddUnique _potentialtargetingactors (.HitActor (Collision|BreakHitResult _array_element))))))
  (return (LocalVariables|GetPotentialTargetingActors)))

(fn FindClosetTarget
  (params (Actors :type Array%20of%20Actor%20Object%20References))
  (for _array_element Actors
    (bind _returnvalue (Collision|LineTraceForObjects (Transformation|GetWorldLocation (Variables|Default|GetCameraRef)) (Transformation|GetActorLocation _array_element) (Utilities|Array|MakeArray "ObjectTypeQuery3") false (Utilities|Array|MakeArray (Components|GetOwner)) "None")) ; A line trace to see if there's a wall or object in the way. Returns true if there isn't.
    (if _returnvalue
      (if (!= (LocalVariables|GetCompareTarget) 0.0)
        (Math|Float|CompareFloat (CallFunction|CheckDistancetoTarget _array_element) (LocalVariables|GetCompareTarget)
          (:==
            _)
          (:<
            _)))
      (LocalVariables|SetCompareTarget (LocalVariables|GetCompareTarget))
      (LocalVariables|SetIdealTarget _array_element)))
  (return (LocalVariables|GetIdealTarget)))

(fn CheckDistancetoTarget
  (params (Target :type Actor%20Object%20Reference))
  (return (- (* (Math|Vector|DotProduct (Math|Vector|Normalize (Transformation|GetActorForwardVector (Variables|Default|GetCharacterRef))) (Math|Vector|Normalize (Math|Rotator|GetRotationXVector (Math|Rotator|FindLookatRotation (Transformation|GetActorLocation Target) (Transformation|GetActorLocation (Variables|Default|GetCharacterRef)))))) (Variables|Default|GetDirectionWeight)) (* (Class|KismetMathLibrary|VectorDistanceSquared (Transformation|GetActorLocation (Variables|Default|GetCharacterRef)) (Transformation|GetActorLocation Target)) (Variables|Default|GetDistanceWeight)))))