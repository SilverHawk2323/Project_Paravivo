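; Melee enemy Blueprint that relies on its parent class for damage, health and death handling.
; Its TakeDamage override calls the parent, then prints the current health as debug output and returns the parent's result.
; The max health, current health and death-check overrides only pass through to the parent.
; The event graph holds only disabled placeholder events, so no melee attack or AI logic lives in these graphs.
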(event EventBeginPlay)

(event Collision|EventActorBeginOverlap
  (params (OtherActor :type Actor%20Object%20Reference)))

(event EventTick
  (params (DeltaSeconds :type Float%20%28single-precision%29)))

(fn ConstructionScript
  (|CallParentFunction))

(fn TakeDamage
  (params (DamageInfo :type S%20Damage%20Info%20Structure) (Damage%20Causer :type Actor%20Object%20Reference))
  (bind _wasdamaged (|CallParentFunction DamageInfo Damage%20Causer))
  (bind _health (CallFunction|GetCurrentHealth))
  (Development|PrintString (Utilities|String|ToString(Float) _health))
  (return _wasdamaged))

(fn GetMaxHealth
  (bind _maxhealth (|CallParentFunction))
  (return _maxhealth))

(fn GetCurrentHealth
  (bind _health (|CallParentFunction))
  (return _health))

(fn IsDead
  (bind _dead (|CallParentFunction))
  (return _dead))