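; Base enemy character that exposes health, team, patrol route, combat range, movement speed and attack functions.
; It uses the Ability System for attributes, a targetable effect applied at BeginPlay, and a melee punch ability.
; BPCDamageSystem handles incoming damage; its bound events play a hit montage or ragdoll the body with a force before destroying it after a delay.
; Heal and ReserveAttackToken are stubs returning zero and false.
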(event Custom|DamageResponse
  (params (Selection :type E_DamageResponse%20Enum :default "NewEnumerator0") (Damage%20Causer :type Actor%20Object%20Reference))
  (switch Utilities|FlowControl|Switch|SwitchonE_DamageResponse Selection
    (:NewEnumerator1
      (Components|Movement|StopMovementImmediately (Variables|Character|GetCharacterMovement))
      (Animation|Montage|PlayMontage (Variables|Character|GetMesh) "/Game/Characters/Mannequins/Anims/Rifle/HitReact/AM_TempHit.AM_TempHit"))))

(event Custom|OnDeath
  (Collision|SetCollisionEnabled (Variables|Default|GetCapsuleComponent) "PhysicsOnly")
  (Pawn|Components|CharacterMovement|DisableMovement (Variables|Character|GetCharacterMovement))
  (Physics|SetSimulatePhysics (Variables|Character|GetMesh) true)
  (Physics|AddForce (Variables|Character|GetMesh) (* (Transformation|GetActorForwardVector) (Variables|Default|GetDeathImpactForce)) "None" true)
  (Utilities|FlowControl|Delay 3.0)
  (Actor|DestroyActor))

(event Custom|Initilize
  (GameplayEffects|ApplyGameplayEffectToSelf (Variables|Default|GetAbilitySystemComponent) "/Game/Blueprint/AbilitySystem/GameplayEffects/GE_SetTargetable.GE_SetTargetable_C" 0.0 (GameplayEffects|MakeEffectContext (Variables|Default|GetAbilitySystemComponent))))

(event EventBeginPlay
  (CallFunction|Initilize))

(event EventAttack
  (Abilities|TryActivateAbilitybyClass (Variables|Default|GetAbilitySystemComponent) "/Game/Blueprint/AbilitySystem/GameplayAbilities/GA_MeleeAttack_Punch.GA_MeleeAttack_Punch_C" true))

(event EventAttackEnd
  (Default|CallOnAttackEnd))

(fn ConstructionScript
  (bind _bpc_damagesystem (Variables|Default|GetBPC_DamageSystem))
  (EventDispatchers|BindEventtoOnDamageResponse _bpc_damagesystem (EventDispatchers|CreateEvent :!event Custom|DamageResponse))
  (EventDispatchers|BindEventtoOnDeath _bpc_damagesystem (EventDispatchers|CreateEvent :!event Custom|OnDeath)))

(fn GetCurrentHealth
  (return (.currentvalue (Variables|/Script/Paravivo.BasicAttributeSet|GetHealth (Variables|Default|GetBasicAttributeSet)))))

(fn GetIdealRange
  (return 1.5e+02 3.5e+02))

(fn GetMaxHealth
  (return (.currentvalue (Variables|/Script/Paravivo.BasicAttributeSet|GetMaxHealth (Variables|Default|GetBasicAttributeSet)))))

(fn GetPatrolRoute
  (return (Variables|AI|GetPatrolRoute)))

(fn GetTeamNumber
  (return (Variables|Combat|GetTeam%20Number)))

(fn Heal
  (params (Amount :type Float%20%28double-precision%29))
  (return 0.0))

(fn IsAttacking
  (return (Variables|/Game/Blueprint/DamageSystem/Attacks/BPC_Attacks.BPC_Attacks_C|GetAttacking (Variables|Default|GetBPC_Attacks))))

(fn IsDead
  (return (Variables|/Game/Blueprint/DamageSystem/BPC_DamageSystem.BPC_DamageSystem_C|GetIsDead (Variables|Default|GetBPC_DamageSystem))))

(fn ReserveAttackToken
  (params (Amount :type Integer))
  (return false))

(fn SetMovementSpeed
  (params (Speed :type E_MovementMode%20Enum :default "NewEnumerator0"))
  (bind _output_get (Variables|/Script/Engine.CharacterMovementComponent|SetMaxWalkSpeed (Variables|Character|GetCharacterMovement) (Utilities|Select :Index Speed :NewEnumerator0 0.0 :NewEnumerator1 2e+02 :NewEnumerator2 5e+02)))
  (return _output_get))

(fn TakeDamage
  (params (DamageInfo :type S%20Damage%20Info%20Structure) (Damage%20Causer :type Actor%20Object%20Reference) (EffectSpecHandle :type Gameplay%20Effect%20Spec%20Handle%20Structure))
  (bind _wasdamaged (Default|TakeDamage (Variables|Default|GetBPC_DamageSystem) DamageInfo Damage%20Causer EffectSpecHandle))
  (return _wasdamaged))