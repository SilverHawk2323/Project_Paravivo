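; BP_EnemyMelee is a melee enemy Blueprint child that relies on its parent for health, damage and death logic.
; On a damage response it briefly tints the mesh's Paint Tint material parameter red, then restores grey after a short delay as a hit flash.
; TakeDamage calls the parent and prints current health to screen for debugging; the other overrides simply forward to the parent.
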(event EventBeginPlay
  (|CallParentFunction))

(event EventDamageResponse
  (params (Selection :type E_DamageResponse%20Enum :default "NewEnumerator0") (Damage%20Causer :type Actor%20Object%20Reference))
  (|CallParentFunction Selection Damage%20Causer)
  (Rendering|Material|SetColorParameterValueonMaterials (Variables|Character|GetMesh) "Paint Tint" "(R=0.640625,G=0.008784,B=0.000000,A=1.000000)")
  (Utilities|FlowControl|Delay 0.1)
  (Rendering|Material|SetColorParameterValueonMaterials (Variables|Character|GetMesh) "Paint Tint" "(R=0.432292,G=0.432292,B=0.432292,A=1.000000)"))

(event EventOnDeath
  (|CallParentFunction))

(fn ConstructionScript
  (|CallParentFunction))

(fn TakeDamage
  (params (DamageInfo :type S%20Damage%20Info%20Structure) (Damage%20Causer :type Actor%20Object%20Reference) (EffectSpecHandle :type Gameplay%20Effect%20Spec%20Handle%20Structure))
  (bind _wasdamaged (|CallParentFunction DamageInfo Damage%20Causer EffectSpecHandle))
  (bind _health (CallFunction|GetCurrentHealth))
  (Development|PrintString (Utilities|String|ToString(Float) _health))
  (return _wasdamaged))

(fn GetMaxHealth
  (bind _maxhealth (|CallParentFunction))
  (return _maxhealth))

(fn GetCurrentHealth
  (bind _health (|CallParentFunction))
  (return _health))

(fn IsDead
  (bind _dead (|CallParentFunction))
  (return _dead))