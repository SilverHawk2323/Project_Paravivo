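; BP_EnemyBase is the enemy base Blueprint, exposing health, damage and combat-state queries.
; Current and max health read from a BasicAttributeSet, while TakeDamage and IsDead delegate to the BPCDamageSystem component.
; Heal, team number, attack state and attack token reservation are stubs returning zero or false, and the event graph and construction script are empty.
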(event EventBeginPlay)

(event Collision|EventActorBeginOverlap
  (params (OtherActor :type Actor%20Object%20Reference)))

(event EventTick
  (params (DeltaSeconds :type Float%20%28single-precision%29)))

(fn ConstructionScript)

(fn GetCurrentHealth
  (return (.currentvalue (Variables|/Script/Paravivo.BasicAttributeSet|GetHealth (Variables|Default|GetBasicAttributeSet)))))

(fn GetMaxHealth
  (return (.currentvalue (Variables|/Script/Paravivo.BasicAttributeSet|GetMaxHealth (Variables|Default|GetBasicAttributeSet)))))

(fn GetTeamNumber
  (return 0))

(fn Heal
  (params (Amount :type Float%20%28double-precision%29))
  (return 0.0))

(fn IsAttacking
  (return false))

(fn IsDead
  (return (Variables|/Game/Blueprint/DamageSystem/BPC_DamageSystem.BPC_DamageSystem_C|GetIsDead (Variables|Default|GetBPC_DamageSystem))))

(fn ReserveAttackToken
  (params (Amount :type Integer))
  (return false))

(fn TakeDamage
  (params (DamageInfo :type S%20Damage%20Info%20Structure) (Damage%20Causer :type Actor%20Object%20Reference))
  (bind _wasdamaged (Default|TakeDamage (Variables|Default|GetBPC_DamageSystem) DamageInfo Damage%20Causer))
  (return _wasdamaged))